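; BP_Grandpy is an actor with a skeletal mesh and a text label that both turn to follow the player.
; The construction script copies DisplayText into the text render component.
; Every tick, the label faces the player and shows only within TextDisplayDistance.
; The mesh rotates on yaw only, with a 90-degree offset, so it stays upright while tracking the player.
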(event `self.ReceiveTick`
  (params (DeltaSeconds :type "Float (single-precision)"))
  (bind _returnvalue (`self.K2_GetActorLocation`))
  (bind _returnvalue_2 (`self.K2_GetActorLocation` (`GameplayStatics.GetPlayerCharacter` 0)))
  (`SceneComponent.SetVisibility` (`self.TextRender`) (<= (`KismetMathLibrary.VSize` (- _returnvalue_2 _returnvalue)) (`self.TextDisplayDistance`)) false)
  (`SceneComponent.K2_SetWorldRotation` (`self.TextRender`) (`KismetMathLibrary.FindLookAtRotation` _returnvalue _returnvalue_2) false false)
  (`SceneComponent.K2_SetWorldRotation` (`self.SkeletalMesh`) (`KismetMathLibrary.MakeRotator` 0.0 0.0 (+ (.yaw (`KismetMathLibrary.FindLookAtRotation` _returnvalue_2 _returnvalue)) 90.0)) false false))

(fn `UserConstructionScript`
  (`TextRenderComponent.K2_SetText` (`self.TextRender`) (`self.DisplayText`)))