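; BP_BadSquare is an enemy that tracks BP_Sammy and bursts into smoke when it dies.
; Sight overlaps set Chasing to Sammy on entry and clear it on exit; this graph contains no movement logic.
; While Dying, Tick checks DeathTimer, which this graph never decrements.
; On expiry it spawns randomly offset and scaled BP_SmokeBall actors, calling DestroyActor inside the spawn loop.
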(event `self.Sight.OnComponentBeginOverlap`
  (params (OverlappedComponent :type "PrimitiveComponent Object Reference") (OtherActor :type "Actor Object Reference") (OtherComp :type "PrimitiveComponent Object Reference") (OtherBodyIndex :type Integer) (bFromSweep :type Boolean) (SweepResult :type "HitResult Structure (by ref)"))
  (bind _asbp_sammy (cast `/Game/Sammy/Blueprints/BP_Sammy` OtherActor))
  (set `self.Chasing` _asbp_sammy))

(event `self.Sight.OnComponentEndOverlap`
  (params (OverlappedComponent :type "PrimitiveComponent Object Reference") (OtherActor :type "Actor Object Reference") (OtherComp :type "PrimitiveComponent Object Reference") (OtherBodyIndex :type Integer))
  (cast `/Game/Sammy/Blueprints/BP_Sammy` OtherActor)
  (set `self.Chasing` null))

(event `self.ReceiveTick`
  (params (DeltaSeconds :type "Float (single-precision)"))
  (bind _smokeballrange (`self.SmokeBallRange`))
  (bind _returnvalue (* _smokeballrange -1.0))
  ;[1 1 1] Kill when death timer runs out and spawn smoke balls.
  (if (`self.Dying`)
    (if (<= (`self.DeathTimer`) 0.0)
      (for _ (range 3)
        (`|SpawnActorFromClass` "/Game/Enemies/BP_SmokeBall.BP_SmokeBall_C" (`KismetMathLibrary.MakeTransform` (+ (`self.K2_GetActorLocation`) (`KismetMathLibrary.MakeVector` (`KismetMathLibrary.RandomFloatInRange` _returnvalue _smokeballrange) (`KismetMathLibrary.RandomFloatInRange` _returnvalue _smokeballrange) (`KismetMathLibrary.RandomFloatInRange` _returnvalue _smokeballrange))) (struct) (* (`self.GetActorScale3D`) (`KismetMathLibrary.RandomFloatInRange` 2.0 4.0))) "Undefined" "OverrideRootScale" null null)
        (`self.K2_DestroyActor`)))))

(fn `UserConstructionScript`)