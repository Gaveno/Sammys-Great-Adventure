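; BP_MushroomPadSnow is a glowing mushroom bounce pad that launches Characters whose capsule overlaps its trigger area.
; On BeginPlay, bounce power and four glow light intensities are multiplied by the length of the mesh's world scale vector.
; Launches are additive, using negated character velocity plus the mesh's up vector times bounce power, so incoming momentum is cancelled and the bounce follows the pad's orientation.
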(event `self.ReceiveBeginPlay`
  (bind _glow1 (`self.Glow1`))
  (bind _glow2 (`self.Glow2`))
  (bind _glow3 (`self.Glow3`))
  (bind _glow4 (`self.Glow4`))
  (set `self.ThisWorldScale` (`KismetMathLibrary.VSize` (`SceneComponent.K2_GetComponentScale` (`self.MushroomMesh`))))
  ;[1 1 1] Bounce power based on world scale
  (set `self.BouncePower` (* (`self.BouncePower`) (`self.ThisWorldScale`)))
  ;[1 1 1] Light Intensity based on world scale
  (`LightComponent.SetIntensity` _glow1 (* (`LightComponentBase.Intensity` _glow1) (`self.ThisWorldScale`)))
  (`LightComponent.SetIntensity` _glow2 (* (`LightComponentBase.Intensity` _glow2) (`self.ThisWorldScale`)))
  (`LightComponent.SetIntensity` _glow3 (* (`LightComponentBase.Intensity` _glow3) (`self.ThisWorldScale`)))
  (`LightComponent.SetIntensity` _glow4 (* (`LightComponentBase.Intensity` _glow4) (`self.ThisWorldScale`))))

(event `self.TriggerArea.OnComponentBeginOverlap`
  (params (OverlappedComponent :type "PrimitiveComponent Object Reference") (OtherActor :type "Actor Object Reference") (OtherComp :type "PrimitiveComponent Object Reference") (OtherBodyIndex :type Integer) (bFromSweep :type Boolean) (SweepResult :type "HitResult Structure (by ref)"))
  ;[1 1 1] Launch Characters that land on top.
  (bind _ascapsule_collision (cast `CapsuleComponent` OtherComp))
  (bind _returnvalue (`ActorComponent.GetOwner` _ascapsule_collision))
  (bind _ascharacter (cast `Character` _returnvalue))
  (`Character.LaunchCharacter` _ascharacter (+ (* (`self.GetVelocity` _returnvalue) -1) (* (`SceneComponent.GetUpVector` (`self.MushroomMesh`)) (`self.BouncePower`))) false false))

(fn `UserConstructionScript`)